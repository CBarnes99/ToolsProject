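; Sphere trigger that stages a handshake weapon handover between the player and a nearby NPC, alongside the TransferItemSequence level sequence.
; An armed player's overlap finds an NPC in the sphere, disables input and AI-moves the NPC to the player's animation reference point.
; A montage notify reattaches the weapon from holder to receiver.
; Completion restores input, resets the DoOnce and walks the NPC back; actor-spawn and binding-tag sequence logic is unused.
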(event `self.Sphere.OnComponentBeginOverlap`
  (params (OverlappedComponent :type "PrimitiveComponent Object Reference") (OtherActor :type "Actor Object Reference") (OtherComp :type "PrimitiveComponent Object Reference") (OtherBodyIndex :type Integer) (bFromSweep :type Boolean) (SweepResult :type "HitResult Structure (by ref)"))
  (bind _asbp_third_person_character (cast `/Game/BP_ThirdPersonCharacter` OtherActor))
  (`/Engine/EditorBlueprintResources/StandardMacros.DoOnce` false :!label _label
    (:`Completed`
      (set `self.Player` _asbp_third_person_character)
      (set `self.bIsPlayer` true)
      (if (`/Game/BP_ThirdPersonCharacter.bHasWeapon` (`self.Player`))
        (for _array_element (`PrimitiveComponent.GetOverlappingActors` (`self.Sphere`) "/Script/Engine.Character")
          (bind _asbp_npc (cast `/Game/BP_NPC` _array_element))
          (bind _output_get (set `self.NPC` _asbp_npc))
          (set `self.bIsNPC` true)
          (set `self.NPC Actor Transform` (`self.GetTransform` _output_get))
          (break))
        (if (and (`self.bIsNPC`) (`self.bIsPlayer`))
          (`KismetSystemLibrary.PrintString` "Both Player and NPC are Present")
          (`self.SpawnLevelSequence`)
          (`self.PlayAnimation`))
        (else
          (`KismetSystemLibrary.PrintString` "Player Doesnt Have Weapon")
          (`self.Finished Animation`))))))

(event `Finished Animation`
  (goto _label :!via `Reset`))

(event `SpawnLevelSequence`
  (bind (_outactor _returnvalue) (`LevelSequencePlayer.CreateLevelSequencePlayer` (`self.TransferItem Sequence`)))
  (add `MovieSceneSequencePlayer.OnFinished` _returnvalue (`|CreateDelegate` :!event `Finished Animation`))
  (`MovieSceneSequencePlayer.Play` _returnvalue))

(event `PlayAnimation`
  (bind _player (`self.Player`))
  (bind _npc (`self.NPC`))
  (bind _npc_2 (`self.NPC`))
  (bind _returnvalue (`KismetSystemLibrary.IsValid` (`self.NPC`)))
  (bind _returnvalue_2 (`KismetSystemLibrary.IsValid` (`self.Player`)))
  (bind _weaponactor (`/Game/BP_ThirdPersonCharacter.WeaponActor` (`self.Player`)))
  (bind _weaponactor_2 (`/Game/BP_NPC.WeaponActor` (`self.NPC`)))
  (bind (_returnvalue_location _returnvalue_rotation) (`KismetMathLibrary.BreakTransform` (`SceneComponent.K2_GetComponentToWorld` (`/Game/BP_ThirdPersonCharacter.AnimationReference` (`self.Player`)))))
  (bind _returnvalue_3 (`KismetSystemLibrary.IsValid` (`/Game/BP_NPC.WeaponActor` (`self.NPC`))))
  (bind _returnvalue_4 (`KismetSystemLibrary.IsValid` (`/Game/BP_ThirdPersonCharacter.WeaponActor` (`self.Player`))))
  (if (and _returnvalue _returnvalue_2)
    (if (xor _returnvalue_4 _returnvalue_3)
      (`|AIMoveTo` _npc_2 _returnvalue_location null
        (:`then`
          (`self.DisableInput` (`self.Player`) (`GameplayStatics.GetPlayerController` 0)))
        (:`OnSuccess`
          (`self.K2_SetActorRotation` _npc_2 _returnvalue_rotation false)
          (`/Engine/EditorBlueprintResources/StandardMacros.IsValid` (`/Game/BP_ThirdPersonCharacter.WeaponActor` (`self.Player`))
            (:`Is Valid`
              (`Character.PlayAnimMontage` (`self.NPC`) "/Game/AM_ShakeHands.AM_ShakeHands" 1.0 "None")
              (bind _notifyname (`|PlayMontage` (`Character.Mesh` (`self.Player`)) "/Game/AM_ShakeHands.AM_ShakeHands")
                (:`OnCompleted`
                  (`self.MontageFinished`))
                (:`OnNotifyBegin`
                  (`KismetSystemLibrary.PrintString` (`KismetStringLibrary.Conv_NameToString` _notifyname))
                  (`/Engine/EditorBlueprintResources/StandardMacros.IsValid` _weaponactor
                    (:`Is Valid`
                      (`self.K2_DetachFromActor` _weaponactor "KeepRelative" "KeepRelative" "KeepRelative")
                      (bind _returnvalue_5 (`self.K2_AttachToComponent` _weaponactor (`Character.Mesh` (`self.NPC`)) "HandGrip_R" "SnapToTarget" "SnapToTarget" "SnapToTarget" true))
                      (if _returnvalue_5
                        (set `/Game/BP_NPC.WeaponActor` (`/Game/BP_ThirdPersonCharacter.WeaponActor` _player) (`self.NPC`))
                        (set `/Game/BP_ThirdPersonCharacter.WeaponActor` null _player)))
                    (:`Is Not Valid`
                      (`KismetSystemLibrary.PrintString` "Weapon Not Valid" true true (struct :`R` 1.0 :`B` 0.062327 :`A` 1.0) 10.0))))))
            (:`Is Not Valid`
              (`Character.PlayAnimMontage` (`self.Player`) "/Game/AM_ShakeHands.AM_ShakeHands" 1.0 "None")
              (bind _notifyname_2 (`|PlayMontage` (`Character.Mesh` (`self.NPC`)) "/Game/AM_ShakeHands.AM_ShakeHands")
                (:`OnCompleted`
                  (`self.MontageFinished`))
                (:`OnNotifyBegin`
                  (`KismetSystemLibrary.PrintString` (`KismetStringLibrary.Conv_NameToString` _notifyname_2))
                  (`/Engine/EditorBlueprintResources/StandardMacros.IsValid` _weaponactor_2
                    (:`Is Valid`
                      (`self.K2_DetachFromActor` _weaponactor_2 "KeepRelative" "KeepRelative" "KeepRelative")
                      (bind _returnvalue_6 (`self.K2_AttachToComponent` _weaponactor_2 (`Character.Mesh` (`self.Player`)) "HandGrip_R" "SnapToTarget" "SnapToTarget" "SnapToTarget" true))
                      (if _returnvalue_6
                        (set `/Game/BP_ThirdPersonCharacter.WeaponActor` (`/Game/BP_NPC.WeaponActor` _npc) (`self.Player`))
                        (set `/Game/BP_NPC.WeaponActor` null _npc)))
                    (:`Is Not Valid`
                      (`KismetSystemLibrary.PrintString` "Weapon Not Valid" true true (struct :`R` 1.0 :`B` 0.062327 :`A` 1.0) 10.0))))))))
        (:`OnFail`
          (`KismetSystemLibrary.PrintString` "Hello")))
      (else
        (`KismetSystemLibrary.PrintString` (`KismetTextLibrary.Conv_TextToString` (`|FormatText` "Either Player Or NPC Both have a weapon, or neither have a weapon: \nPlayer - {player} \nNPC - {NPC}" _returnvalue_4 _returnvalue_3)) true true (struct :`R` 1.0 :`G` 0.008341 :`A` 1.0) 10.0)))
    (else
      (`KismetSystemLibrary.PrintString` (`KismetTextLibrary.Conv_TextToString` (`|FormatText` "Either Player Or NPC isnt valid: \nPlayer - {player} \nNPC - {NPC}" _returnvalue _returnvalue_2)) true true (struct :`R` 1.0 :`G` 0.008341 :`A` 1.0) 10.0))))

(event `MontageFinished`
  (bind _npc (`self.NPC`))
  (bind (_npc_actor_transform_location _npc_actor_transform_rotation) (`KismetMathLibrary.BreakTransform` (`self.NPC Actor Transform`)))
  (`self.EnableInput` (`self.Player`) (`GameplayStatics.GetPlayerController` 0))
  (`self.Finished Animation`)
  (`|AIMoveTo` _npc _npc_actor_transform_location null
    (:`OnSuccess`
      (`self.K2_SetActorRotation` _npc _npc_actor_transform_rotation false))))

(fn `UserConstructionScript`)